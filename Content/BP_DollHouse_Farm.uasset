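; Interactive doll house puzzle that mirrors the real toilet and heating rooms, opened with a key on its keyhole.
; Its miniature doors close and block or unblock the linked real doors, and door states persist through JSON save/load.
; A crowbar toy placed by interaction or Tick overlap checks snaps into place and teleports its real counterpart to the matching room.
; Removing the toy resets that counterpart, while taking the crowbar hides the toy.
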(event OnChangeMovingState(ToiletDoor)
  (params (NewState :type EMovingState%20Enum :default "MS_OPEN"))
  (bind _realdoor_toilet (Variables|Default|GetRealDoor_Toilet))
  ;[1 1 1] Блокирование / разблокирование реальных дверей дверками
  (switch Utilities|FlowControl|Switch|SwitchonEMovingState NewState
    (:MS_OPEN
      (Utilities|IsValid _realdoor_toilet
        (:Is%20Valid
          (Class|Door|SetBlock _realdoor_toilet false))))
    (:MS_CLOSE
      (Utilities|IsValid _realdoor_toilet
        (:Is%20Valid
          (if (Utilities|Enum|NotEqual(Enum) (Variables|/Script/HelloNeighbor.Door|Getm_eState _realdoor_toilet) "DS_CLOSE")
            (Class|Door|SetDoorState _realdoor_toilet "DS_CLOSING" 0 0.0)))))))

(event OnChangeMovingState(HeatingDoor)
  (params (NewState :type EMovingState%20Enum :default "MS_OPEN"))
  (bind _realdoor_heating (Variables|Default|GetRealDoor_Heating))
  ;[1 1 1] Блокирование / разблокирование реальных дверей дверками
  (switch Utilities|FlowControl|Switch|SwitchonEMovingState NewState
    (:MS_OPEN
      (Utilities|IsValid _realdoor_heating
        (:Is%20Valid
          (Class|Door|SetBlock _realdoor_heating false))))
    (:MS_CLOSE
      (Utilities|IsValid _realdoor_heating
        (:Is%20Valid
          (if (Utilities|Enum|NotEqual(Enum) (Variables|/Script/HelloNeighbor.Door|Getm_eState _realdoor_heating) "DS_CLOSE")
            (Class|Door|SetDoorState _realdoor_heating "DS_CLOSING" 0 0.0)))))))

(event OnComponentEndOverlap(HeaterCollision)
  (params (OverlappedComponent :type Primitive%20Component%20Object%20Reference) (OtherActor :type Actor%20Object%20Reference) (OtherComp :type Primitive%20Component%20Object%20Reference) (OtherBodyIndex :type Integer))
  (Utilities|Casting|CastToBP_CrowbarToy OtherActor)
  (Utilities|FlowControl|Delay 0.4)
  (Variables|Default|SetToy 0)
  (Transformation|SetActorTransform (Variables|Default|GetRealToy) (Variables|Default|GetRealToyStartingTransform) false true))

(event OnComponentEndOverlap(ToiletCollision)
  (params (OverlappedComponent :type Primitive%20Component%20Object%20Reference) (OtherActor :type Actor%20Object%20Reference) (OtherComp :type Primitive%20Component%20Object%20Reference) (OtherBodyIndex :type Integer))
  (Utilities|Casting|CastToBP_CrowbarToy OtherActor)
  (Utilities|FlowControl|Delay 0.4)
  (Variables|Default|SetToy 0)
  (Transformation|SetActorTransform (Variables|Default|GetRealToy) (Variables|Default|GetRealToyStartingTransform) false true))

(event Custom|CrowbarTaken
  (bind _toy (Variables|Default|GetToy))
  (bind _flatcomponent (Variables|/Script/HelloNeighbor.FlatActor|GetFlatComponent _toy))
  ;[1 1 1] Взяли лом => игрушку больше брать нельзя, лом у игрушки исчезает из рук
  (Utilities|IsValid _toy
    (:Is%20Valid
      (Class|FlatComponent|SetMode _flatcomponent "FM_Hold")
      (Class|FlatComponent|SetFlatType _flatcomponent "FT_Static")
      (Rendering|SetVisibility (Variables|/Game/Act2/BP_CrowbarToy.BP_CrowbarToy_C|GetStaticMesh1 _toy) false false))))

(event Custom|OnRealHeatingChangeState
  (params (NewState :type EDoorState%20Enum :default "DS_OPEN"))
  ;[1 1 1] Реальная дверь закрылась и игрушечная "заблокирована" - заблокировать реальную дверь
  (switch Utilities|FlowControl|Switch|SwitchonEDoorState NewState
    (:DS_CLOSE
      (Class|Door|SetBlock (Variables|Default|GetRealDoor_Heating) (Utilities|Enum|Equal(Enum) (Class|MovingComponent|GetMovingState (Variables|Default|GetHeatingDoor)) "MS_CLOSE")))))

(event Custom|OnRealToiletChangeState
  (params (NewState :type EDoorState%20Enum :default "DS_OPEN"))
  ;[1 1 1] Реальная дверь закрылась и игрушечная "заблокирована" - заблокировать реальную дверь
  (switch Utilities|FlowControl|Switch|SwitchonEDoorState NewState
    (:DS_CLOSE
      (Class|Door|SetBlock (Variables|Default|GetRealDoor_Toilet) (Utilities|Enum|Equal(Enum) (Class|MovingComponent|GetMovingState (Variables|Default|GetToiletDoor)) "MS_CLOSE")))))

(event EventTick
  (params (DeltaSeconds :type Float%20%28single-precision%29))
  (bind _toy (Variables|Default|GetToy))
  (bind _bufertoycomponent (Variables|Default|GetBuferToyComponent))
  (bind _buferspawnactor (Variables|Default|GetBuferSpawnActor))
  (bind _rootcomponent (Variables|/Script/Engine.Actor|GetRootComponent _toy))
  (Utilities|IsValid (Variables|Default|GetToy)
    (:Is%20Not%20Valid
      (Utilities|FlowControl|Sequence
        (:then_0
          (CallFunction|CheckToyCollision (Variables|Default|GetToiletCollision)))
        (:then_1
          (CallFunction|CheckToyCollision (Variables|Default|GetHeaterCollision))))
      ;[1 1 1] Если тыкнули игрушкой на туалет или объект в бойлерной
      (Utilities|IsValid _toy
        (:Is%20Valid
          (Transformation|AttachActorToActor _toy self "None" "KeepWorld" "KeepWorld" "KeepRelative" true)
          (Transformation|SetRelativeTransform _rootcomponent (Math|Transform|MakeTransform (Variables|/Script/Engine.SceneComponent|GetRelativeLocation _bufertoycomponent) (Variables|/Script/Engine.SceneComponent|GetRelativeRotation _bufertoycomponent) (Variables|/Script/Engine.SceneComponent|GetRelativeScale3D (Variables|Default|Gettoilet))) false false)
          (bind _asprimitive_component (Utilities|Casting|CastToPrimitiveComponent _rootcomponent))
          (Physics|SetSimulatePhysics _asprimitive_component false)
          (Utilities|IsValid _buferspawnactor
            (:Is%20Valid
              (CallFunction|SpawnRealToy (Transformation|GetActorTransform _buferspawnactor)))))))))

(event EventOnPostLoad
  (bind _realdoor_heating (Variables|Default|GetRealDoor_Heating))
  (bind _realdoor_toilet (Variables|Default|GetRealDoor_Toilet))
  (EventDispatchers|AssignWasTaken (Variables|Default|GetCrowbar) (delegate Custom|CrowbarTaken))
  (EventDispatchers|AssignOnChangeState _realdoor_heating (delegate Custom|OnRealHeatingChangeState))
  (EventDispatchers|AssignOnChangeState _realdoor_toilet (delegate Custom|OnRealToiletChangeState))
  (Utilities|FlowControl|Sequence
    (:then_0
      ;[1 1 1] Реальная дверь закрылась и игрушечная "заблокирована" - заблокировать реальную дверь
      (Class|Door|SetBlock _realdoor_heating (Utilities|Enum|Equal(Enum) (Class|MovingComponent|GetMovingState (Variables|Default|GetHeatingDoor)) "MS_CLOSE")))
    (:then_1
      (Class|Door|SetBlock _realdoor_toilet (Utilities|Enum|Equal(Enum) (Class|MovingComponent|GetMovingState (Variables|Default|GetToiletDoor)) "MS_CLOSE")))))

(event EventOnEventAction
  (params (ActionMaker :type Actor%20Object%20Reference) (SpecialComponent :type Primitive%20Component%20Object%20Reference))
  (bind _toiletdoor (Variables|Default|GetToiletDoor))
  (bind _toiletdoor_2 (Variables|Default|GetToiletDoor))
  (bind _heatingdoor (Variables|Default|GetHeatingDoor))
  (bind _heatingdoor_2 (Variables|Default|GetHeatingDoor))
  ;[1 1 1] Блокирование / разблокирование реальных дверей дверками
  (if (== SpecialComponent _toiletdoor_2)
    (switch Utilities|FlowControl|Switch|SwitchonEMovingState (Class|MovingComponent|GetMovingState _toiletdoor_2)
      (:MS_OPEN
        (Class|MovingComponent|SetMovingState _toiletdoor "MS_CLOSING" :!label _label))
      (:MS_CLOSE
        (Class|MovingComponent|SetMovingState _toiletdoor "MS_OPENING" :!label _label_2)
        (Audio|Components|Audio|Play (Variables|Default|Getmetal_hit_17_Cue) 0.0 :!label _label_3))
      (:MS_OPENING
        (goto _label))
      (:MS_CLOSING
        (goto _label_2)))
    (elif (== SpecialComponent _heatingdoor)
      (switch Utilities|FlowControl|Switch|SwitchonEMovingState (Class|MovingComponent|GetMovingState _heatingdoor)
        (:MS_OPEN
          _)
        (:MS_CLOSE
          (Class|MovingComponent|SetMovingState _heatingdoor_2 "MS_OPENING" :!label _label_4)
          (goto _label_3))
        (:MS_OPENING
          _)
        (:MS_CLOSING
          (goto _label_4)))
      (Class|MovingComponent|SetMovingState _heatingdoor_2 "MS_CLOSING"))))

(event EventOnApplytoMe
  (params (Character :type Character%20Object%20Reference) (ApplyActor :type Flat%20Actor%20Object%20Reference) (IntersectComponent :type Primitive%20Component%20Object%20Reference))
  ;[1 1 1] Если тыкнули ключиком на замочную скавжину
  (if (Math|Boolean|ANDBoolean (== (Utilities|GetClass ApplyActor) "/Game/Objects/BP_Objects/BP_DollHouseKey.BP_DollHouseKey_C") (== IntersectComponent (Variables|Default|GetKeyhole)) (Utilities|Enum|Equal(Enum) (Class|MovingComponent|GetMovingState (Variables|Default|GetDoor1)) "MS_CLOSE"))
    (Audio|Components|Audio|Play (Variables|Default|Getlock_open_Cue) 0.0)
    (Utilities|FlowControl|Delay 0.5)
    (Audio|Components|Audio|Play (Variables|Default|Getdoor_opening_lite_Cue) 0.0)
    (Class|MovingComponent|SetMovingState (Variables|Default|GetDoor1) "MS_OPENING")
    (Class|MovingComponent|SetMovingState (Variables|Default|GetDoor2) "MS_OPENING")
    (else
      ;[1 1 1] Если тыкнули игрушкой на туалет или объект в бойлерной
      (bind _asbp_crowbar_toy (Utilities|Casting|CastToBP_CrowbarToy ApplyActor))
      (Variables|Default|SetToy _asbp_crowbar_toy)
      (if (and (== (Utilities|GetClass ApplyActor) "/Game/Act2/BP_CrowbarToy.BP_CrowbarToy_C") (or (== IntersectComponent (Variables|Default|Gettoilet)) (== IntersectComponent (Variables|Default|GetBOX))))
        (bind _returnvalue (Class|Human|FindHuman))
        (Class|Human|SetHandsState _returnvalue "HS_FAST_THROW")
        (Audio|Components|Audio|Play (Variables|Default|Getsuitcase_open_Cue) 0.0)
        (if (== (Variables|Default|Gettoilet) IntersectComponent)
          (Variables|Default|SetBuferSpawnActor (Variables|Default|GetRealToiletActorPosition))
          (Variables|Default|SetBuferToyComponent (Variables|Default|GetToiletToyPosition))
          (else
            (Variables|Default|SetBuferSpawnActor (Variables|Default|GetRealHeatingActorPosition))
            (Variables|Default|SetBuferToyComponent (Variables|Default|GetHeatingToyPosition))))
        (Utilities|IsValid (Variables|Default|GetToy)
          (:Is%20Valid
            (Transformation|AttachActorToActor (Variables|Default|GetToy) self "None" "KeepWorld" "KeepWorld" "KeepRelative" true)
            (Transformation|SetRelativeTransform (Variables|/Script/Engine.Actor|GetRootComponent (Variables|Default|GetToy)) (Math|Transform|MakeTransform (Variables|/Script/Engine.SceneComponent|GetRelativeLocation (Variables|Default|GetBuferToyComponent)) (Variables|/Script/Engine.SceneComponent|GetRelativeRotation (Variables|Default|GetBuferToyComponent)) (Variables|/Script/Engine.SceneComponent|GetRelativeScale3D (Variables|Default|Gettoilet))) false false)
            (bind _asprimitive_component (Utilities|Casting|CastToPrimitiveComponent (Variables|/Script/Engine.Actor|GetRootComponent (Variables|Default|GetToy))))
            (Physics|SetSimulatePhysics _asprimitive_component false)
            (Utilities|IsValid (Variables|Default|GetBuferSpawnActor)
              (:Is%20Valid
                (CallFunction|SpawnRealToy (Transformation|GetActorTransform (Variables|Default|GetBuferSpawnActor)))))))))))

(event EventOnLoad
  (params (JsonObject :type JSON%20Structure))
  (bind _toiletdoor (Variables|Default|GetToiletDoor))
  (bind _heatingdoor (Variables|Default|GetHeatingDoor))
  ;[1 1 1] Загрузка
  (bind (_boolvalue _returnvalue) (Class|JSONLibrary|GetValueasBool JsonObject "DollHouseDoorState"))
  (if _returnvalue
    (if _boolvalue
      (Class|MovingComponent|SetMovingState (Variables|Default|GetDoor1) "MS_OPEN")
      (Class|MovingComponent|SetMovingState (Variables|Default|GetDoor2) "MS_OPEN")
      (else
        (Class|MovingComponent|SetMovingState (Variables|Default|GetDoor1) "MS_CLOSE")
        (Class|MovingComponent|SetMovingState (Variables|Default|GetDoor2) "MS_CLOSE")))
    (bind _boolvalue_2 (Class|JSONLibrary|GetValueasBool JsonObject "DollHouseRealDoorToilet"))
    (if _boolvalue_2
      (Class|MovingComponent|SetMovingState _toiletdoor "MS_OPEN")
      (else
        (Class|MovingComponent|SetMovingState _toiletdoor "MS_CLOSE")))
    (bind _boolvalue_3 (Class|JSONLibrary|GetValueasBool JsonObject "DollHouseRealDoorHeating"))
    (if _boolvalue_3
      (Class|MovingComponent|SetMovingState _heatingdoor "MS_OPEN")
      (else
        (Class|MovingComponent|SetMovingState _heatingdoor "MS_CLOSE")))))

(fn ConstructionScript)

(fn OnIsActionComponent
  (params (Component :type Primitive%20Component%20Object%20Reference))
  (bind _returnvalue (Class|Human|FindHuman))
  (bind _returnvalue_2 (Class|Human|GetInventory _returnvalue))
  (return (Math|Boolean|ORBoolean (== Component (Variables|Default|GetKeyhole)) (== Component (Variables|Default|GetToiletDoor)) (== Component (Variables|Default|GetHeatingDoor)) (and (== (Utilities|GetClass (Class|Inventory|GetCurrentObject _returnvalue_2)) "/Game/Act2/BP_CrowbarToy.BP_CrowbarToy_C") (or (== Component (Variables|Default|Gettoilet)) (== Component (Variables|Default|GetBOX)))))))

(fn OnSave
  (params (JsonObject :type JSON%20Structure))
  (Class|JSONLibrary|SetValueasBool JsonObject "DollHouseDoorState" (Utilities|Enum|Equal(Enum) (Class|MovingComponent|GetMovingState (Variables|Default|GetDoor1)) "MS_OPEN"))
  (Class|JSONLibrary|SetValueasBool JsonObject "DollHouseRealDoorToilet" (Utilities|Enum|Equal(Enum) (Class|MovingComponent|GetMovingState (Variables|Default|GetToiletDoor)) "MS_OPEN"))
  (Class|JSONLibrary|SetValueasBool JsonObject "DollHouseRealDoorHeating" (Utilities|Enum|Equal(Enum) (Class|MovingComponent|GetMovingState (Variables|Default|GetHeatingDoor)) "MS_OPEN")))

(fn SpawnRealToy
  (params (ActorTransform :type Transform))
  (bind (_location _rotation) (Math|Transform|BreakTransform ActorTransform))
  (bind _realtoy (Variables|Default|GetRealToy))
  (Utilities|IsValid _realtoy
    (:Is%20Valid
      (Transformation|SetWorldLocationAndRotation (Variables|/Script/Engine.Actor|GetRootComponent _realtoy) _location _rotation false false)
      (Physics|SetSimulatePhysics (Variables|/Game/Act2/BP_RealCrowbarToy.BP_RealCrowbarToy_C|GetStaticMesh _realtoy) false)
      (Class|FlatComponent|SetFlatType (Variables|/Script/HelloNeighbor.FlatActor|GetFlatComponent _realtoy) "FT_Movable"))))

(fn CheckToyCollision
  (params (OverlappedBox :type Box%20Component%20Object%20Reference))
  (bind _overlappingactors (Collision|GetOverlappingActors OverlappedBox "/Game/Act2/BP_CrowbarToy.BP_CrowbarToy_C" :!class /Script/Engine.PrimitiveComponent))
  (if (> (Utilities|Array|Length _overlappingactors) 0)
    (bind _asbp_crowbar_toy (Utilities|Casting|CastToBP_CrowbarToy (Utilities|Array|Get(acopy) _overlappingactors)))
    (if (Utilities|Enum|Equal(Enum) (Variables|/Script/HelloNeighbor.FlatComponent|GetMode (Variables|/Script/HelloNeighbor.FlatActor|GetFlatComponent _asbp_crowbar_toy)) "FM_Free")
      (Variables|Default|SetToy _asbp_crowbar_toy)
      (if (== OverlappedBox (Variables|Default|GetToiletCollision))
        (Variables|Default|SetBuferSpawnActor (Variables|Default|GetRealToiletActorPosition))
        (Variables|Default|SetBuferToyComponent (Variables|Default|GetToiletToyPosition))
        (else
          (Variables|Default|SetBuferSpawnActor (Variables|Default|GetRealHeatingActorPosition))
          (Variables|Default|SetBuferToyComponent (Variables|Default|GetHeatingToyPosition))))
      (return))))